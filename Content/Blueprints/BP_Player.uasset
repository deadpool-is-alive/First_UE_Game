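; BP_Player is the player Character Blueprint, providing WASD movement, mouse look and jumping.
; Raw W, A, S and D key events set forward and right axis values, reset to zero on release.
; Tick turns them into movement input along the camera's forward and right vectors.
; Mouse input drives controller yaw and inverted-Y pitch, and Space triggers Jump.
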(event EventBeginPlay)

(event Collision|EventActorBeginOverlap
  (params (OtherActor :type Actor%20Object%20Reference)))

(event EventTick
  (params (DeltaSeconds :type Float%20%28single-precision%29))
  (Pawn|Input|AddMovementInput (+ (* (Math|Vector|GetForwardVector (Variables|Default|GetCamera)) (Variables|Default|GetForward%20Axis)) (* (Math|Vector|GetRightVector (Variables|Default|GetCamera)) (Variables|Default|GetRightAxis))) 1.0 false))

(event Input|KeyboardEvents|D
  (params (Key :type Key%20Structure :default "None"))
  (:Pressed
    (Variables|Default|SetRightAxis 1.0))
  (:Released
    (Variables|Default|SetRightAxis 0.0)))

(event Input|KeyboardEvents|A
  (params (Key :type Key%20Structure :default "None"))
  (:Pressed
    (Variables|Default|SetRightAxis -1.0))
  (:Released
    (Variables|Default|SetRightAxis 0.0)))

(event Input|KeyboardEvents|W
  (params (Key :type Key%20Structure :default "None"))
  (:Pressed
    (Variables|Default|SetForward%20Axis 1.0))
  (:Released
    (Variables|Default|SetForward%20Axis 0.0)))

(event Input|KeyboardEvents|S
  (params (Key :type Key%20Structure :default "None"))
  (:Pressed
    (Variables|Default|SetForward%20Axis -1.0))
  (:Released
    (Variables|Default|SetForward%20Axis 0.0)))

(event Input|KeyboardEvents|SpaceBar
  (params (Key :type Key%20Structure :default "None"))
  (:Pressed
    (Character|Jump)))

(event Input|MouseEvents|LeftMouseButton
  (params (Key :type Key%20Structure :default "None")))

(event Input|MouseEvents|Mouse2D
  (params (AxisValue :type Vector :default "0, 0, 0"))
  (bind (_x _y) (Math|Vector|BreakVector AxisValue))
  (Pawn|Input|AddControllerYawInput _x)
  (Pawn|Input|AddControllerPitchInput (* _y -1.0)))

(fn ConstructionScript)